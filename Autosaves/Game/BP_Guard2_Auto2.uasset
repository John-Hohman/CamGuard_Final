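; Guard AI pawn that investigates a camera-supplied location, walks the supplied patrol points, then returns to its BeginPlay location.
; Investigate feeds Patrol, which loops through AIMoveTo calls and one-second delays on the immediate exec pin, so steps advance without waiting for arrival.
; Index is never reset after a patrol.
; PawnSensing triggers an empty Chase event, and the move-to-player-and-return logic is left unconnected.
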(event `self.ReceiveBeginPlay`
  (set `self.Start Location` (`SceneComponent.K2_GetComponentLocation` (`self.CapsuleComponent`))))

(event `Investigate`
  (params (Destination :type "Vector Structure") (`Patrol Points` :type "Array of Actor Object Reference"))
  (set `self.Patrol Points` `Patrol Points`)
  (`|AIMoveTo` self Destination null
    (:`then`
      (`KismetSystemLibrary.Delay` 1.0)
      (`self.Patrol`))))

(event `Patrol`
  (`|AIMoveTo` self (0.0 0.0 0.0) (`|GetArrayItem` (`self.Patrol Points`) (`self.Index`)) 100.0 :!label _label
    (:`then`
      (`KismetSystemLibrary.Delay` 1.0)
      (`/Engine/EditorBlueprintResources/StandardMacros.IncrementInt` (`self.Index`)
        (:`  `
          (if (>= (`self.Index`) (`KismetArrayLibrary.Array_Length` (`self.Patrol Points`)))
            (`self.Return to Guard Station`)
            (else
              (goto _label))))))))

(event `Return to Guard Station`
  (`|AIMoveTo` self (`self.Start Location`) null 100.0))

(event `Chase`)

(event `self.PawnSensing.OnSeePawn`
  (params (Pawn :type "Pawn Object Reference"))
  (`self.Chase`))

(fn `UserConstructionScript`)