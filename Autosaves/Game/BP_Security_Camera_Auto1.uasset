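; Security camera actor that spots the first-person player through AI Perception and calls in guards.
; On detection it waits briefly, rechecks the stimulus, then calls Investigate on every BP_Guard2, passing its PatrolPoints and a zero destination.
; Debug boxes and prints mark alerts and lost sightings, while PawnSensing events only print.
; Older BP_Guard logic matching guards to CameraValue is left unconnected.
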(event `self.ReceiveBeginPlay`
  (`ActorComponent.Activate` (`self.PawnSensing`) false))

(event `self.PawnSensing.OnSeePawn`
  (params (Pawn :type "Pawn Object Reference"))
  (`KismetSystemLibrary.PrintString` "I can see a pawn"))

(event `self.PawnSensing.OnComponentActivated`
  (params (Component :type "ActorComponent Object Reference") (bReset :type Boolean))
  (`KismetSystemLibrary.PrintString` "Hello"))

(event `self.AIPerception.OnTargetPerceptionUpdated`
  (params (Actor :type "Actor Object Reference") (Stimulus :type "AIStimulus Structure"))
  (bind (_age _expirationage _strength _stimuluslocation _receiverlocation _tag _bsuccessfullysensed) (break `AIStimulus` Stimulus))
  ;[1 1 1] Camera Alerting Guard
  (bind _asbp_first_person_character (cast `/Game/FirstPerson/Blueprints/BP_FirstPersonCharacter` Actor))
  (if _bsuccessfullysensed
    (`KismetSystemLibrary.PrintString` "Enemy Spotted")
    (`KismetSystemLibrary.Delay` 1.0)
    (if _bsuccessfullysensed
      (`KismetSystemLibrary.PrintString` "Calling Guards")
      (bind _returnvalue (`SceneComponent.K2_GetComponentLocation` (`Character.CapsuleComponent` _asbp_first_person_character)))
      (`KismetSystemLibrary.DrawDebugBox` _returnvalue (0.0 0.0 0.0) (struct :`R` 1.0 :`A` 1.0))
      (bind _outactors (`GameplayStatics.GetAllActorsOfClass` "/Game/ThirdPerson/Blueprints/BP_Guard2.BP_Guard2_C"))
      (for _array_element _outactors
        (`/Game/ThirdPerson/Blueprints/BP_Guard2.Investigate` _array_element (0.0 0.0 0.0) (`self.Patrol Points`))))
    (else
      (`KismetSystemLibrary.PrintString` "Enemy Lost")
      (`KismetSystemLibrary.DrawDebugBox` _returnvalue (0.0 0.0 0.0) (struct :`R` 1.0 :`A` 1.0)))))

(fn `UserConstructionScript`)