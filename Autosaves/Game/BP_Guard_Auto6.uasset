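; BP_Guard is an AI guard pawn with a scripted patrol and a tag-on-touch check against the player.
; Investigate, Point1 and Point2 chain delayed AI Move To calls to one shared hard-coded location, then ReturnToBase sends the guard to a second location.
; Chase sets a flag but its move has no target, and the pawn-sensing event is empty.
; A box overlap with BP_FirstPersonCharacter prints a tag message.
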(event `Investigate`
  ;[1 1 1] Guard Movement
  (`KismetSystemLibrary.Delay` 1.0)
  (`|AIMoveTo` self (1900.0 -70.0 88.0) null 100.0
    (:`OnSuccess`
      (`self.Point 1`))))

(event `Point 1`
  ;[1 1 1] Guard Movement
  (`KismetSystemLibrary.Delay` 1.0)
  (`|AIMoveTo` self (1900.0 -70.0 88.0) null 100.0
    (:`OnSuccess`
      (`self.Point 2`))))

(event `Point 2`
  ;[1 1 1] Guard Movement
  (`KismetSystemLibrary.Delay` 1.0)
  (`|AIMoveTo` self (1900.0 -70.0 88.0) null 100.0
    (:`then`
      (`self.Return to Base`))))

(event `Return to Base`
  ;[1 1 1] Guard Movement
  (`KismetSystemLibrary.Delay` 1.0)
  (`|AIMoveTo` self (-1150.0 -70.0 108.0) null 100.0))

(event `Chase`
  (set `self.Chasing` true)
  (`|AIMoveTo` self (0.0 0.0 0.0) null))

(event `self.PawnSensing.OnSeePawn`
  (params (Pawn :type "Pawn Object Reference")))

(event `self.Box.OnComponentBeginOverlap`
  (params (OverlappedComponent :type "PrimitiveComponent Object Reference") (OtherActor :type "Actor Object Reference") (OtherComp :type "PrimitiveComponent Object Reference") (OtherBodyIndex :type Integer) (bFromSweep :type Boolean) (SweepResult :type "HitResult Structure (by ref)"))
  (cast `/Game/FirstPerson/Blueprints/BP_FirstPersonCharacter` OtherActor)
  (`KismetSystemLibrary.PrintString` "TAG! You're it!"))

(fn `UserConstructionScript`)