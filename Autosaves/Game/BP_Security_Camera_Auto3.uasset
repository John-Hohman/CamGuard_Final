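; Security camera that alerts its linked guards when it perceives the first-person player character.
; AI Perception updates drive a FlipFlop alternating spotted and lost, rather than reading the sensed state.
; On spotted, it calls Investigate on every BP_Guard whose GaurdValue matches its CameraValue; both branches have debug prints and boxes.
; PawnSensing handlers are empty, and return-to-base and BP_Guard2 group-alert logic are disconnected.
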(event `self.ReceiveBeginPlay`
  (`ActorComponent.Activate` (`self.PawnSensing`) false))

(event `self.PawnSensing.OnSeePawn`
  (params (Pawn :type "Pawn Object Reference")))

(event `self.PawnSensing.OnComponentActivated`
  (params (Component :type "ActorComponent Object Reference") (bReset :type Boolean)))

(event `self.AIPerception.OnTargetPerceptionUpdated`
  (params (Actor :type "Actor Object Reference") (Stimulus :type "AIStimulus Structure"))
  ;[1 1 1] Camera Alerting Guard
  (cast `/Game/FirstPerson/Blueprints/BP_FirstPersonCharacter` Actor)
  (if true
    (`/Engine/EditorBlueprintResources/StandardMacros.FlipFlop`
      (:`A`
        (`KismetSystemLibrary.PrintString` "Enemy Spotted")
        (bind _outactors (`GameplayStatics.GetAllActorsOfClass` "/Game/BP_Guard.BP_Guard_C"))
        (for _array_element _outactors
          (if (== (`/Game/BP_Guard.Gaurd Value` _array_element) (`self.Camera Value`))
            (`/Game/BP_Guard.Investigate` _array_element)
            (`KismetSystemLibrary.Delay` 1.0)
            (if true
              (`KismetSystemLibrary.PrintString` "Calling Guards")
              (`KismetSystemLibrary.DrawDebugBox` (0.0 0.0 0.0) (0.0 0.0 0.0) (struct :`R` 1.0 :`A` 1.0) :!label _label)))))
      (:`B`
        (`KismetSystemLibrary.PrintString` "Enemy Lost")
        (goto _label)))))

(fn `UserConstructionScript`)