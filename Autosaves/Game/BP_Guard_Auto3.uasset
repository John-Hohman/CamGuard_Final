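; Guard AI pawn that investigates, chases seen pawns and catches the first-person player.
; Investigate starts a one-pass chain of delayed AIMoveTo steps through hardcoded points, ending back at a base location.
; PawnSensing triggers a chase to the seen pawn's current location, then resumes the route at Point1 whether the move succeeds or fails.
; A box overlap calls Caught on the player, then resets them to a checkpoint after a short delay.
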(event `self.Box.OnComponentBeginOverlap`
  (params (OverlappedComponent :type "PrimitiveComponent Object Reference") (OtherActor :type "Actor Object Reference") (OtherComp :type "PrimitiveComponent Object Reference") (OtherBodyIndex :type Integer) (bFromSweep :type Boolean) (SweepResult :type "HitResult Structure (by ref)"))
  (cast `/Game/FirstPerson/Blueprints/BP_FirstPersonCharacter` OtherActor)
  (bind _asbp_first_person_character (cast `/Game/FirstPerson/Blueprints/BP_FirstPersonCharacter` (`GameplayStatics.GetPlayerCharacter` 0)))
  (`/Game/FirstPerson/Blueprints/BP_FirstPersonCharacter.Caught` _asbp_first_person_character)
  (`KismetSystemLibrary.Delay` 1.5)
  (`/Game/FirstPerson/Blueprints/BP_FirstPersonCharacter.Reset to Checkpoint` _asbp_first_person_character))

(event `self.ReceiveBeginPlay`)

(event `Investigate`
  ;[1 1 1] Guard Movement
  (`KismetSystemLibrary.Delay` 1.0)
  (`|AIMoveTo` self (-320.0 -3930.0 88.0) null 100.0
    (:`OnSuccess`
      (`self.Point 1`))))

(event `Point 1`
  ;[1 1 1] Guard Movement
  (`KismetSystemLibrary.Delay` 1.0)
  (`|AIMoveTo` self (140.0 -3930.0 88.0) null 100.0
    (:`OnSuccess`
      (`self.Point 2`))))

(event `Point 2`
  ;[1 1 1] Guard Movement
  (`KismetSystemLibrary.Delay` 1.0)
  (`|AIMoveTo` self (-840.0 -3930.0 88.0) null 100.0
    (:`OnSuccess`
      (`self.Return to Base`))))

(event `Return to Base`
  ;[1 1 1] Guard Movement
  (`KismetSystemLibrary.Delay` 1.0)
  (`|AIMoveTo` self (-280.0 -1570.0 88.0) null 100.0))

(event `Chase`
  (set `self.Chasing` true)
  (`|AIMoveTo` self (`self.K2_GetActorLocation` (stale `self.PawnSensing.OnSeePawn` Pawn)) null
    (:`OnSuccess`
      _)
    (:`OnFail`
      _))
  (set `self.Chasing` false)
  (`self.Point 1`))

(event `self.PawnSensing.OnSeePawn`
  (params (Pawn :type "Pawn Object Reference"))
  (`self.Chase`))

(fn `UserConstructionScript`)