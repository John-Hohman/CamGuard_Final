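; Guard AI that investigates, patrols and chases the player, using PawnSensing and AIMoveTo.
; A camera calls Investigate with a destination and patrol points; Patrol steps through them toward a return to the start location, gated on the Chasing flag.
; Seeing a pawn triggers Chase, which falls back to Patrol when the move ends.
; A Delay loop polls player distance for a tag, which only prints messages and fades the screen.
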(event `self.ReceiveBeginPlay`
  (bind _returnvalue (`GameplayStatics.GetPlayerCameraManager` 0))
  ;[1 1 1] Getting Player
  (set `self.Start Location` (`SceneComponent.K2_GetComponentLocation` (`self.CapsuleComponent`)))
  (if (<= (`KismetMathLibrary.Vector_Distance` (`SceneComponent.K2_GetComponentLocation` (`self.CapsuleComponent`)) (`SceneComponent.K2_GetComponentLocation` (`Character.CapsuleComponent` (`GameplayStatics.GetPlayerCharacter` 0)))) 100.0) :!label _label
    (`KismetSystemLibrary.PrintString` "TAG!!!!!!!")
    (`PlayerCameraManager.StartCameraFade` :`self` _returnvalue :`ToAlpha` 1.0 :`Duration` 1.0 :`bShouldFadeAudio` true)
    (`KismetSystemLibrary.PrintString` "Moving to last checkpoint")
    (`PlayerCameraManager.StartCameraFade` :`self` _returnvalue)
    (else
      (`KismetSystemLibrary.Delay` 0.2)
      (goto _label))))

(event `Investigate`
  (params (Destination :type "Vector Structure") (`Patrol Points` :type "Array of Actor Object Reference"))
  ;[1 1 1] Debugging
  (if (`self.Debugging`)
    (`TextRenderComponent.K2_SetText` (`self.TextRender`) (`KismetTextLibrary.Conv_StringToText` "Investigate")))
  (set `self.Patrol Points` `Patrol Points`)
  (set `self.Index` 0)
  (`|AIMoveTo` self Destination null 100.0
    (:`OnSuccess`
      (`KismetSystemLibrary.Delay` 1.0)
      (if (`self.Chasing`)
        (`self.Patrol`)))))

(event `Patrol`
  ;[1 1 1] Debugging
  (if (`self.Debugging`)
    (`TextRenderComponent.K2_SetText` (`self.TextRender`) (`KismetTextLibrary.Conv_StringToText` "Patrol")))
  (`|AIMoveTo` self (0.0 0.0 0.0) (`|GetArrayItem` (`self.Patrol Points`) (`self.Index`)) 100.0 :!label _label_2
    (:`OnSuccess`
      _)
    (:`OnFail`
      _))
  (`KismetSystemLibrary.Delay` 1.0)
  (`/Engine/EditorBlueprintResources/StandardMacros.IncrementInt` (`self.Index`)
    (:`  `
      (if (`self.Chasing`)
        (if (>= (`self.Index`) (`KismetArrayLibrary.Array_Length` (`self.Patrol Points`)))
          (`self.Return to Guard Station`)
          (else
            (goto _label_2)))))))

(event `Return to Guard Station`
  ;[1 1 1] Debugging
  (if (`self.Debugging`)
    (`TextRenderComponent.K2_SetText` (`self.TextRender`) (`KismetTextLibrary.Conv_StringToText` "Return to Guard Station")))
  (`|AIMoveTo` self (`self.Start Location`) null 100.0))

(event `Chase`
  ;[1 1 1] Debugging
  (if (`self.Debugging`)
    (`TextRenderComponent.K2_SetText` (`self.TextRender`) (`KismetTextLibrary.Conv_StringToText` "Chase")))
  (set `self.Chasing` true)
  (bind _movementresult (`|AIMoveTo` self (`self.K2_GetActorLocation` (stale `self.PawnSensing.OnSeePawn` Pawn)) null)
    (:`OnSuccess`
      _)
    (:`OnFail`
      _))
  (switch `EPathFollowingResult` _movementresult
    (:`Success`
      (`KismetSystemLibrary.PrintString` "We are at the player's last known location"))
    (:`Blocked`
      _)
    (:`OffPath`
      _)
    (:`Invalid`
      _))
  (set `self.Chasing` false) ; No More Chasing
  (`self.Patrol`))

(event `self.PawnSensing.OnSeePawn`
  (params (Pawn :type "Pawn Object Reference"))
  (`self.Chase`))

(fn `UserConstructionScript`)