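; BP_Security_Camera is a work-in-progress security camera that detects the player and is meant to alert guards.
; AI Perception updates print sight gained or lost, re-checking the same stimulus after a short delay before printing a guard call.
; Both paths draw a debug box at the stimulus location and loop over all BP_Gaurd actors, but the loop body is empty.
; A Pawn Sensing component, activated on BeginPlay, only prints debug messages.
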(event `self.ReceiveBeginPlay`
  (`ActorComponent.Activate` (`self.PawnSensing`) false))

(event `self.PawnSensing.OnSeePawn`
  (params (Pawn :type "Pawn Object Reference"))
  (`KismetSystemLibrary.PrintString` "I can see a pawn"))

(event `self.PawnSensing.OnComponentActivated`
  (params (Component :type "ActorComponent Object Reference") (bReset :type Boolean))
  (`KismetSystemLibrary.PrintString` "Hello"))

(event `self.AIPerception.OnTargetPerceptionUpdated`
  (params (Actor :type "Actor Object Reference") (Stimulus :type "AIStimulus Structure"))
  (bind (_age _expirationage _strength _stimuluslocation _receiverlocation _tag _bsuccessfullysensed) (break `AIStimulus` Stimulus))
  (if _bsuccessfullysensed
    (`KismetSystemLibrary.PrintString` "see player")
    (`KismetSystemLibrary.Delay` 1.0)
    (if _bsuccessfullysensed
      (`KismetSystemLibrary.PrintString` "call the gaurds")
      (`KismetSystemLibrary.DrawDebugBox` _stimuluslocation :!label _label)
      (bind _outactors (`GameplayStatics.GetAllActorsOfClass` "/Game/BP_Gaurd.BP_Gaurd_C"))
      (for _array_element _outactors
        _))
    (else
      (`KismetSystemLibrary.PrintString` "lost sight")
      (goto _label))))

(fn `UserConstructionScript`)